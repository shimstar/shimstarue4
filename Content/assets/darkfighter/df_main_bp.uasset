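; Dark fighter pawn Blueprint that handles damage from green bullets and its own death.
; TakeDamage subtracts the damage value of a green_bullet_bp from Health, ignoring other bullet types.
; At zero health it calls DestroyPawn on its playerController_game_bp controller, then destroys itself, which only happens if that controller cast succeeds.
; Event graph and construction script are empty.
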(event `self.ReceiveBeginPlay`)

(event `self.ReceiveActorBeginOverlap`
  (params (OtherActor :type "Actor Object Reference")))

(event `self.ReceiveTick`
  (params (DeltaSeconds :type "Float (single-precision)")))

(fn `take damage`
  (params (Bullet :type "Actor Object Reference"))
  (bind _asgreen_bullet_bp (cast `/Game/bp/green_bullet_bp` Bullet))
  (bind _output_get (set `self.Health` (- (`self.Health`) (`/Game/bp/green_bullet_bp.damage` _asgreen_bullet_bp))))
  (if (<= _output_get 0.0)
    (bind _asplayer_controller_game_bp (cast `/Game/bp/playerController_game_bp` (`self.GetController`)))
    (`/Game/bp/playerController_game_bp.destroy_pawn` _asplayer_controller_game_bp)
    (`self.K2_DestroyActor`)))

(fn `UserConstructionScript`)