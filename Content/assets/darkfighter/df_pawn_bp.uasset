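; Player-controlled Dark Fighter ship pawn with server-authoritative, physics-driven flight.
; Clients forward speed and steering-torque input to the server, which applies forces and pushes the transform back every tick, with client physics disabled.
; The server also zeroes speed on hits, subtracts bullet damage and destroys the pawn at zero health.
; Clients scale engine glow with speed and add other ships to the HUD radar with an approach sound.
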(event `SetLocation Event`
  (params (location :type "Vector Structure") (rotation :type "Rotator Structure"))
  ;[0.1568 1 0.08294] replicate location to client
  (`SceneComponent.K2_SetWorldLocationAndRotation` (`self.StaticMesh`) location rotation false false))

(event `self.ReceiveTick`
  (params (DeltaSeconds :type "Float (single-precision)"))
  (bind _staticmesh (`self.StaticMesh`))
  (bind _staticmesh_2 (`self.StaticMesh`))
  (`/Engine/EditorBlueprintResources/ActorMacros.Switch Has Authority`
    (:`Authority`
      (`|ExecutionSequence`
        (:`then_0`
          ;[0.2949 1 0.1977] move Forward
          (`PrimitiveComponent.AddForce` _staticmesh (* (`SceneComponent.GetForwardVector` _staticmesh) (* (`self.speed`) -1.0)) "None" true))
        (:`then_1`
          ;[0.1568 1 0.08294] replicate location to client
          (`self.SetLocation Event` (`SceneComponent.K2_GetComponentLocation` _staticmesh_2) (`SceneComponent.K2_GetComponentRotation` _staticmesh_2)))))
    (:`Remote`
      (`|ExecutionSequence`
        (:`then_0`
          ;[1 0.8398 0.0346] Glowing engine depending on speed
          (bind _output_get (set `self.prcentspeed` (/ (`self.speed`) (`self.speedmax`))))
          (bind _asmaterial_instance_dynamic (cast `MaterialInstanceDynamic` (`PrimitiveComponent.GetMaterial` (`self.StaticMesh`) 0)))
          (`MaterialInstanceDynamic.SetScalarParameterValue` _asmaterial_instance_dynamic "p_emissive" (* _output_get 25.0)))))))

(event `self.ReceiveBeginPlay`
  ;[1 1 1] disable physic on client
  (`/Engine/EditorBlueprintResources/ActorMacros.Switch Has Authority`
    (:`Remote`
      ;[1 0.1676 0.7039] Add player to radar
      (`|ExecutionSequence`
        (:`then_0`
          (if (not (`self.IsLocallyControlled` self))
            (bind _ashudgame (cast `/Game/game/hudgame` (`PlayerController.GetHUD` (`GameplayStatics.GetPlayerController` 0))))
            (`/Game/game/hudgame.addToRadar` _ashudgame self)
            (`GameplayStatics.PlaySound2D` "/Game/assets/sounds/playerapproach.playerapproach")))
        (:`then_1`
          (`PrimitiveComponent.SetSimulatePhysics` (`self.StaticMesh`) false)
          (`PrimitiveComponent.CreateDynamicMaterialInstance` (`self.StaticMesh`) 0 "/Game/assets/darkfighter/dark_fighter_7_Inst.dark_fighter_7_Inst"))))))

(event `changeSpeedServer`
  (params (speed :type "Float (double-precision)"))
  ;[0.3047 0.5326 1] speed
  (set `self.speed` speed))

(event `InputAxis|speed`
  (params (AxisValue :type "Float (single-precision)"))
  (bind _returnvalue (+ (`self.speed`) (* AxisValue 15.0)))
  ;[0.3047 0.5326 1] speed
  (`/Engine/EditorBlueprintResources/ActorMacros.Switch Has Authority`
    (:`Remote`
      (if (<= _returnvalue (`self.speedmax`))
        (if (>= _returnvalue -150.0)
          (bind _output_get (set `self.speed` _returnvalue))
          (`self.changeSpeedServer` _output_get))))))

(event `InputAxis|leftright`
  (params (AxisValue :type "Float (single-precision)"))
  ;[0.2064 0.1899 1] manage torque
  (`/Engine/EditorBlueprintResources/ActorMacros.Switch Has Authority`
    (:`Remote`
      (`self.ADDtorque_Event` (* (`SceneComponent.GetUpVector` (`self.StaticMesh`)) (* AxisValue 3.0))))))

(event `self.ReceiveActorBeginOverlap`
  (params (OtherActor :type "Actor Object Reference"))
  ;[1 1 1] Collision
  (`/Engine/EditorBlueprintResources/ActorMacros.Switch Has Authority`
    (:`Authority`
      (if (>= (`KismetStringLibrary.FindSubstring` (`KismetSystemLibrary.GetDisplayName` OtherActor) "bullet") 0)
        (bind _asgreen_bullet_bp (cast `/Game/bp/green_bullet_bp` OtherActor))
        (bind _output_get (set `self.health` (- (`self.health`) (`/Game/bp/green_bullet_bp.damage` _asgreen_bullet_bp))))
        (if (<= _output_get 0.0)
          (bind _asplayer_controller_game_bp (cast `/Game/bp/playerController_game_bp` (`self.GetController` self)))
          (`/Game/bp/playerController_game_bp.destroy_pawn` _asplayer_controller_game_bp)
          (`self.K2_DestroyActor` self))))))

(event `ADDtorque_Event`
  (params (val :type "Vector Structure"))
  ;[0.2064 0.1899 1] manage torque
  (`/Engine/EditorBlueprintResources/ActorMacros.Switch Has Authority`
    (:`Authority`
      (`PrimitiveComponent.AddTorque` (`self.StaticMesh`) val "None" true))))

(event `InputAxis|updwon`
  (params (AxisValue :type "Float (single-precision)"))
  ;[0.2064 0.1899 1] manage torque
  (`/Engine/EditorBlueprintResources/ActorMacros.Switch Has Authority`
    (:`Remote`
      (`self.ADDtorque_Event` (* (`SceneComponent.GetRightVector` (`self.StaticMesh`)) (* AxisValue 3.0))))))

(event `self.ReceiveHit`
  (params (MyComp :type "PrimitiveComponent Object Reference") (Other :type "Actor Object Reference") (OtherComp :type "PrimitiveComponent Object Reference") (bSelfMoved :type Boolean) (HitLocation :type "Vector Structure") (HitNormal :type "Vector Structure") (NormalImpulse :type "Vector Structure") (Hit :type "HitResult Structure (by ref)"))
  ;[1 1 1] Speed 0 on hit
  (`/Engine/EditorBlueprintResources/ActorMacros.Switch Has Authority`
    (:`Authority`
      (set `self.speed` 0.0))))

(fn `UserConstructionScript`)