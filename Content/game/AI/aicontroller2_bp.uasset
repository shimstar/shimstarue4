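; AI controller that flies a df_pawnai_bp pawn between gopoint actors with physics and shoots along the way, running on server Tick.
; It ramps speed while pushing the mesh along negative forward, replicates its transform, and switches to the first other gopoint when within 500 units.
; The target's local-space position drives yaw, then pitch torque, a Demitour U-turn flag, and delayed Red_bullet_bp spawning once aligned.
; Debug prints remain active.
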(event `self.ReceiveBeginPlay`)

(event `self.ReceiveTick`
  (params (DeltaSeconds :type "Float (single-precision)"))
  (bind _returnvalue (* DeltaSeconds 5.0))
  (bind _speed (`self.speed`))
  (bind _targettogo (`self.targetToGo`))
  (bind _distance (`self.distance`))
  (bind _returnvalue_2 (* (`self.distance`) -1.0))
  (`/Engine/EditorBlueprintResources/ActorMacros.Switch Has Authority`
    (:`Authority`
      (`|ExecutionSequence`
        (:`then_0`
          (if (`KismetSystemLibrary.IsValid` _targettogo)
            ;[0.598 0.9617 1] transformation coord relative de la cible
            (bind _asdf_pawnai_bp (cast `/Game/game/AI/df_pawnai_bp` (`self.K2_GetPawn`)))
            (bind _asgopoint (cast `/Game/game/zone/gopoint` _targettogo))
            (`self.calcDistance` _asdf_pawnai_bp _asgopoint)
            ;[1 1 1] Change target when too near
            (if (> (`self.distance`) 500.0)
              ;[0.8051 1 0.1456] speed up
              (if (< _speed (`self.speedmax`))
                (set `self.speed` (+ _speed 40.0)))
              (else
                (`self.changeTarget`)))
            (else
              ;[1 0.6283 0.2793] New target si null
              (`self.changeTarget`))))
        (:`then_1`
          ;[0.2195 1 0.1947] move forward
          (bind _asdf_pawnai_bp_2 (cast `/Game/game/AI/df_pawnai_bp` (`self.K2_GetPawn`)))
          (bind _staticmesh (`/Game/game/AI/df_pawnai_bp.StaticMesh` _asdf_pawnai_bp_2))
          (`PrimitiveComponent.AddForce` _staticmesh (* (`SceneComponent.GetForwardVector` _staticmesh) (* (`self.speed`) -1.0)) "None" true))
        (:`then_2`
          ;[1 0.8719 0.08169] REplication
          (bind _asdf_pawnai_bp_3 (cast `/Game/game/AI/df_pawnai_bp` (`self.K2_GetPawn`)))
          (`/Game/game/AI/df_pawnai_bp.replicateTransform` _asdf_pawnai_bp_3 (`SceneComponent.K2_GetComponentToWorld` (`/Game/game/AI/df_pawnai_bp.StaticMesh` _asdf_pawnai_bp_3))))
        (:`then_3`
          (if (`self.demitour`)
            (bind _asdf_pawnai_bp_4 (cast `/Game/game/AI/df_pawnai_bp` (`self.K2_GetPawn`) :!label _label))
            (bind _staticmesh_2 (`/Game/game/AI/df_pawnai_bp.StaticMesh` _asdf_pawnai_bp_4))
            (`PrimitiveComponent.AddTorque` _staticmesh_2 (* (`SceneComponent.GetUpVector` _staticmesh_2) _returnvalue) "None" true)
            (bind _returnvalue_3 (`KismetMathLibrary.InverseTransformLocation` (`SceneComponent.K2_GetComponentToWorld` (`/Game/game/AI/df_pawnai_bp.StaticMesh` _asdf_pawnai_bp)) (`SceneComponent.K2_GetComponentLocation` (`/Game/game/zone/gopoint.StaticMesh` _asgopoint))))
            (bind _x (.x _returnvalue_3))
            (bind _y (.y _returnvalue_3))
            (bind _z (.z _returnvalue_3))
            (if (< (- _returnvalue_2 1000.0) _x)
              (if (> (+ _returnvalue_2 1000.0) _x)
                (set `self.demitour` false)))
            (elif (!= _distance 0.0)
              (if (< _x 0.0)
                _
                (elif (< (- _distance 1000.0) _x)
                  (if (> (+ _distance 1000.0) _x)
                    (set `self.demitour` true)
                    (goto _label)
                    (else
                      _))))
              ;[0.1861 0.3558 1] Torque horizontal si abs(y) > 50
              (if (> (`KismetMathLibrary.Abs` _y) 100.0)
                (bind _asdf_pawnai_bp_5 (cast `/Game/game/AI/df_pawnai_bp` (`self.K2_GetPawn`)))
                (bind _staticmesh_3 (`/Game/game/AI/df_pawnai_bp.StaticMesh` _asdf_pawnai_bp_5))
                (`PrimitiveComponent.AddTorque` _staticmesh_3 (* (`SceneComponent.GetUpVector` _staticmesh_3) (* _returnvalue (select `bool` (> _y 0.0) :`false` 1.0 :`true` -1.0 :!type "Float (single-precision)"))) "None" true)
                (else
                  ;[0.3003 0.3115 1] Torque vertical si abs(z) > 50
                  (if (> (`KismetMathLibrary.Abs` _z) 100.0)
                    (bind _asdf_pawnai_bp_6 (cast `/Game/game/AI/df_pawnai_bp` (`self.K2_GetPawn`)))
                    (bind _staticmesh_4 (`/Game/game/AI/df_pawnai_bp.StaticMesh` _asdf_pawnai_bp_6))
                    (`PrimitiveComponent.AddTorque` _staticmesh_4 (* (`SceneComponent.GetRightVector` _staticmesh_4) (* _returnvalue (`KismetMathLibrary.SelectFloat` 1.0 -1.0 (> _z 0.0)))) "None" true)
                    (else
                      (`KismetSystemLibrary.Delay` 0.2)
                      (bind _asdf_pawnai_bp_7 (cast `/Game/game/AI/df_pawnai_bp` (`self.K2_GetPawn`)))
                      (bind _staticmesh_5 (`/Game/game/AI/df_pawnai_bp.StaticMesh` _asdf_pawnai_bp_7))
                      (`|SpawnActorFromClass` "/Game/game/red_bullet_bp.red_bullet_bp_C" (`KismetMathLibrary.MakeTransform` (+ (`SceneComponent.K2_GetComponentLocation` _staticmesh_5) (* (`KismetMathLibrary.GetForwardVector` (`SceneComponent.K2_GetComponentRotation` _staticmesh_5)) 50.0))) "AlwaysSpawn" "OverrideRootScale" self))))))))
        (:`then_4`
          ;[1 0.208 0.802] Print vector relatif de la target
          (`KismetSystemLibrary.PrintString` (`KismetStringLibrary.Concat_StrStr` (`KismetStringLibrary.Concat_StrStr` (`KismetStringLibrary.Concat_StrStr` (`KismetStringLibrary.Concat_StrStr` (`KismetStringLibrary.Conv_VectorToString` _returnvalue_3) (`KismetSystemLibrary.GetDisplayName` (`self.targetToGo`))) (`KismetStringLibrary.Conv_DoubleToString` (`self.distance`))) "//") (`KismetStringLibrary.Conv_BoolToString` (`self.demitour`)))))))))

(fn `calcDistance`
  (params (pawn :type "/Game/game/AI/df_pawnai_bp Object Reference") (target :type "/Game/game/zone/gopoint Object Reference"))
  (bind _x (.x (- (`SceneComponent.K2_GetComponentLocation` (`/Game/game/AI/df_pawnai_bp.StaticMesh` pawn)) (`SceneComponent.K2_GetComponentLocation` (`/Game/game/zone/gopoint.StaticMesh` target)))))
  (bind _y (.y (- (`SceneComponent.K2_GetComponentLocation` (`/Game/game/AI/df_pawnai_bp.StaticMesh` pawn)) (`SceneComponent.K2_GetComponentLocation` (`/Game/game/zone/gopoint.StaticMesh` target)))))
  (bind _z (.z (- (`SceneComponent.K2_GetComponentLocation` (`/Game/game/AI/df_pawnai_bp.StaticMesh` pawn)) (`SceneComponent.K2_GetComponentLocation` (`/Game/game/zone/gopoint.StaticMesh` target)))))
  (set `self.distance` (`KismetMathLibrary.Sqrt` (+ (+ (* _x _x) (* _y _y)) (* _z _z))))
  (return))

(fn `changeTarget`
  (bind _targettogo (`self.targetToGo`))
  (bind _outactors (`GameplayStatics.GetAllActorsOfClass` "/Game/game/zone/gopoint.gopoint_C"))
  (for _array_element _outactors
    (`KismetSystemLibrary.PrintString` (`KismetStringLibrary.Concat_StrStr` (`KismetStringLibrary.Concat_StrStr` (`KismetSystemLibrary.GetDisplayName` _array_element) "//") (`KismetSystemLibrary.GetDisplayName` _targettogo)))
    (if (!= _array_element _targettogo)
      (set `self.targetToGo` _array_element)
      (break))))

(fn `UserConstructionScript`)