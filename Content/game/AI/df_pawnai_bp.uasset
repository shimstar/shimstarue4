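; Enemy dark-fighter AI pawn that shows on the player's radar and takes damage from green bullets.
; On clients, spawning registers it with the HUD radar, plays a spotted sound and creates a life bar, and destruction removes both radar entry and bar.
; Every Tick passes the mesh's world transform through a custom replication event.
; TakeDamage subtracts bullet damage from Health and destroys the pawn at zero; no AI decision logic lives here.
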(event `self.ReceiveBeginPlay`
  (`/Engine/EditorBlueprintResources/ActorMacros.Switch Has Authority`
    (:`Remote`
      ;[0.3928 0.3605 1] add To radar
      (`|ExecutionSequence`
        (:`then_0`
          (bind _ashudgame (cast `/Game/game/ui/hudgame` (`PlayerController.GetHUD` (`GameplayStatics.GetPlayerController` 0))))
          (`/Game/game/ui/hudgame.addToRadar` _ashudgame self)
          (`GameplayStatics.PlaySound2D` "/Game/assets/sounds/ennemyspotted.ennemyspotted")
          (bind _returnvalue (`|CreateWidget` "/Game/game/ui/lifeaibar.lifeaibar_C"))
          (`UserWidget.AddToViewport` _returnvalue 0)
          (bind _output_get (set `self.lifebar` _returnvalue))
          (set `/Game/game/ui/lifeaibar.owner` self _output_get))
        (:`then_1`
          (`PrimitiveComponent.CreateDynamicMaterialInstance` (`self.StaticMesh`) 0 "/Game/assets/darkfighter/dark_fighter_7_Inst.dark_fighter_7_Inst"))))))

(event `replicate Movement`
  (params (location :type "Vector Structure") (rotation :type "Rotator Structure"))
  (`SceneComponent.K2_SetWorldLocationAndRotation` (`self.StaticMesh`) location rotation false false))

(event `self.ReceiveActorBeginOverlap`
  (params (OtherActor :type "Actor Object Reference")))

(event `replicateTransform`
  (params (transform :type "Transform Structure"))
  (`SceneComponent.K2_SetWorldTransform` (`self.StaticMesh`) transform false false))

(event `self.ReceiveTick`
  (params (DeltaSeconds :type "Float (single-precision)"))
  (`self.replicateTransform` (`SceneComponent.K2_GetComponentToWorld` (`self.StaticMesh`))))

(event `self.ReceiveDestroyed`
  (`/Engine/EditorBlueprintResources/ActorMacros.Switch Has Authority`
    (:`Remote`
      (`Widget.RemoveFromParent` (`self.lifebar`))
      (bind _ashudgame (cast `/Game/game/ui/hudgame` (`PlayerController.GetHUD` (`GameplayStatics.GetPlayerController` 0))))
      (`/Game/game/ui/hudgame.removeFromRadar` _ashudgame self))))

(fn `Take Damage`
  (params (Bullet :type "Actor Object Reference"))
  (bind _asgreen_bullet_bp (cast `/Game/game/green_bullet_bp` Bullet))
  (bind _output_get (set `self.Health` (- (`self.Health`) (`/Game/game/green_bullet_bp.damage` _asgreen_bullet_bp))))
  (if (<= _output_get 0.0)
    (`self.K2_DestroyActor`)))

(fn `UserConstructionScript`)