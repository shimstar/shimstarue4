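; AI controller that drives a physics-based df_pawnai_bp pawn between gopoint actors, running on the server.
; Each tick pushes the mesh along its forward axis, steers with torques from the target direction in local space, and adjusts Speed by distance.
; On arrival, ChangeTarget takes the first differently named gopoint, effectively alternating between two.
; Transforms pass to the pawn's ReplicateMovement after a short delay; GetSteering is unused scaffolding.
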(event `self.ReceiveBeginPlay`)

(event `self.ReceiveTick`
  (params (DeltaSeconds :type "Float (single-precision)"))
  (bind _speedmax (`self.speedmax`))
  (bind _speed (`self.speed`))
  (`/Engine/EditorBlueprintResources/ActorMacros.Switch Has Authority`
    (:`Authority`
      (bind _asdf_pawnai_bp (cast `/Game/assets/darkfighter/df_pawnai_bp` (`self.K2_GetPawn`)))
      (`|ExecutionSequence`
        (:`then_0`
          (bind _staticmesh (`/Game/assets/darkfighter/df_pawnai_bp.StaticMesh` _asdf_pawnai_bp))
          ;[1 1 1] move forward
          (`PrimitiveComponent.AddForce` _staticmesh (* (`SceneComponent.GetForwardVector` _staticmesh) (* (`self.speed`) -1.0)) "None" true))
        (:`then_1`
          ;[1 1 1] Manage Relative direction looking at target
          (if (`KismetSystemLibrary.IsValid` (`self.targetToGo`))
            (bind _asgopoint (cast `/Game/bp/gopoint` (`self.targetToGo`)))
            (bind _asdf_pawnai_bp_2 (cast `/Game/assets/darkfighter/df_pawnai_bp` (`self.K2_GetPawn`)))
            (`|ExecutionSequence`
              (:`then_0`
                (bind _staticmesh_2 (`/Game/assets/darkfighter/df_pawnai_bp.StaticMesh` _asdf_pawnai_bp_2))
                (bind _returnvalue (`SceneComponent.K2_GetComponentLocation` _staticmesh_2))
                (bind _returnvalue_2 (`SceneComponent.K2_GetComponentLocation` (`/Game/bp/gopoint.StaticMesh` _asgopoint)))
                (bind _z (.z (`KismetMathLibrary.LessLess_VectorRotator` (`KismetMathLibrary.GetDirectionVector` _returnvalue _returnvalue_2) (`SceneComponent.K2_GetComponentRotation` _staticmesh_2))))
                (if (< (`KismetMathLibrary.Abs` (.x (`KismetMathLibrary.LessLess_VectorRotator` (`KismetMathLibrary.GetDirectionVector` _returnvalue _returnvalue_2) (`SceneComponent.K2_GetComponentRotation` _staticmesh_2)))) 0.99)
                  ;[1 1 1] torque up
                  (`PrimitiveComponent.AddTorque` _staticmesh (* (`SceneComponent.GetUpVector` _staticmesh) (* DeltaSeconds 10.0)) "None" true)))
              (:`then_1`
                (if (> (`KismetMathLibrary.Abs` _z) 0.05)
                  ;[1 1 1] Torque left
                  (`PrimitiveComponent.AddTorque` _staticmesh (* (`SceneComponent.GetRightVector` _staticmesh) (* (`KismetMathLibrary.SelectFloat` 10.0 -10.0 (> _z 0.0)) DeltaSeconds)) "None" true)))
              (:`then_2`
                (bind _returnvalue_3 (`KismetMathLibrary.VSize` (- _returnvalue _returnvalue_2)))
                ;[1 1 1] Manage speed
                (if (> _returnvalue_3 1000.0)
                  (if (< _speed _speedmax)
                    (set `self.speed` (+ _speed 40.0) :!label _label))
                  (elif (> _returnvalue_3 500.0)
                    (if (< _speed (/ _speedmax 2.0))
                      (goto _label))
                    (else
                      (set `self.speed` 0.0)
                      ;[0 1 0.08472] near the target, change the taget7
                      (`self.changeTarget`)))))
              (:`then_4`
                ;[1 0.2362 0.8226] Launch movement replication
                (bind _asdf_pawnai_bp_3 (cast `/Game/assets/darkfighter/df_pawnai_bp` (`self.K2_GetPawn`)))
                (`KismetSystemLibrary.Delay` 0.02)
                (bind _staticmesh_3 (`/Game/assets/darkfighter/df_pawnai_bp.StaticMesh` _asdf_pawnai_bp_3))
                (`/Game/assets/darkfighter/df_pawnai_bp.replicate Movement` _asdf_pawnai_bp_3 (`SceneComponent.K2_GetComponentLocation` _staticmesh_3) (`SceneComponent.K2_GetComponentRotation` _staticmesh_3))))
            (else
              ;;[1 0.15 0.15] target is null
              (`self.changeTarget`))))))))

(fn `changeTarget`
  (bind _targettogo (`self.targetToGo`))
  (bind _outactors (`GameplayStatics.GetAllActorsOfClass` "/Game/bp/gopoint.gopoint_C"))
  (for _array_element _outactors
    (if (`KismetSystemLibrary.IsValid` _targettogo)
      (bind _asgopoint (cast `/Game/bp/gopoint` _targettogo))
      (if (`KismetStringLibrary.NotEqual_StrStr` (`KismetSystemLibrary.GetDisplayName` _array_element) (`KismetSystemLibrary.GetDisplayName` _asgopoint))
        (set `self.targetToGo` _array_element)
        (break))
      (else
        (set `self.targetToGo` _array_element)
        (break))))
  (return))

(fn `getSteering`
  (params (target :type "Actor Object Reference"))
  (returns (x :type "Float (double-precision)") (y :type "Float (double-precision)") (z :type "Float (double-precision)"))
  (bind _outactors (`GameplayStatics.GetAllActorsOfClass` "/Game/bp/gopoint.gopoint_C")))

(fn `UserConstructionScript`)