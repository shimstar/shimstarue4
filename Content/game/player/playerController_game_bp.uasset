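; Player controller for a networked pawn shooter, handling spawn and respawn, firing, death UI and view toggle.
; Authority spawns and possesses a df_pawn_bp above the first PlayerStart at random height, while remote clients create the HUD and crosshair.
; Holding left mouse opens a Tick gate throttled by Delay, sending mesh- or cursor-based aim to a server event that spawns bullets.
; The view axis toggles mesh visibility; Escape quits.
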(event `InputAxis|changeView`
  (params (AxisValue :type "Float (single-precision)"))
  (`KismetSystemLibrary.Delay` 0.2)
  (if (> AxisValue 0.0)
    (bind _asdf_pawn_bp (cast `/Game/game/player/df_pawn_bp` (`self.K2_GetPawn`)))
    (if (== (`self.view`) 0)
      (set `self.view` 1)
      (bind _staticmesh (`/Game/game/player/df_pawn_bp.StaticMesh` _asdf_pawn_bp))
      (`SceneComponent.SetVisibility` _staticmesh true false)
      (else
        (set `self.view` 0)
        (`SceneComponent.SetVisibility` _staticmesh false false)))))

(event `spawn new pawn`
  ;[1 1 1] Spawn first pawn and pawn after death
  (`/Engine/EditorBlueprintResources/ActorMacros.Switch Has Authority` :!label _label
    (:`Authority`
      (bind _outactors (`GameplayStatics.GetAllActorsOfClass` "/Script/Engine.PlayerStart"))
      (for _array_element _outactors
        (bind _returnvalue (`|SpawnActorFromClass` "/Game/game/player/df_pawn_bp.df_pawn_bp_C" (`KismetMathLibrary.MakeTransform` (+ (`self.K2_GetActorLocation` _array_element) (`KismetMathLibrary.MakeVector` 0.0 0.0 (`KismetMathLibrary.RandomFloatInRange` 0.0 1000.0)))) "Undefined" "OverrideRootScale" self))
        (`self.Possess` _returnvalue)
        (break))
      (`self.hide mortui`))))

(event `hide mortui`
  ;[1 1 1] Remove Mort UI on spawn
  (bind _foundwidgets (`WidgetBlueprintLibrary.GetAllWidgetsOfClass` "/Game/game/ui/ui_death_widget.ui_death_widget_C"))
  (for _array_element _foundwidgets
    (`Widget.RemoveFromParent` _array_element)
    (set `self.bShowMouseCursor` false)))

(event `self.ReceiveBeginPlay`
  ;[1 1 1] Spawn first pawn and pawn after death
  (`|ExecutionSequence`
    (:`then_0`
      (goto _label))
    (:`then_1`
      (`/Engine/EditorBlueprintResources/ActorMacros.Switch Has Authority`
        (:`Remote`
          (bind _returnvalue (`|CreateWidget` "/Game/game/ui/game_widget.game_widget_C" self))
          (`UserWidget.AddToViewport` _returnvalue 0)
          (set `self.bShowMouseCursor` true)
          (if (`self.tircentre`)
            (bind _returnvalue_2 (`|CreateWidget` "/Game/game/ui/viseur.viseur_C" self))
            (`UserWidget.AddToViewport` _returnvalue_2 0)
            (else
              (set `self.CurrentMouseCursor` "Crosshairs"))))))))

(event `self.ReceiveTick`
  (params (DeltaSeconds :type "Float (single-precision)"))
  (`|ExecutionSequence`
    (:`then_0`
      ;[0.2484 0.1438 1] fire on left mouse click
      (`/Engine/EditorBlueprintResources/StandardMacros.Gate` true :!label _label_2
        (:`Exit`
          (`KismetSystemLibrary.Delay` 0.2)
          (bind _asdf_pawn_bp (cast `/Game/game/player/df_pawn_bp` (`self.K2_GetPawn`)))
          (bind _staticmesh (`/Game/game/player/df_pawn_bp.StaticMesh` _asdf_pawn_bp))
          (bind _returnvalue (`SceneComponent.K2_GetComponentRotation` _staticmesh))
          (bind _camera (`/Game/game/player/df_pawn_bp.Camera` _asdf_pawn_bp))
          (bind _returnvalue_2 (`SceneComponent.K2_GetComponentLocation` _camera))
          (`self.fireserver_Event` (`KismetMathLibrary.MakeTransform` (+ (`SceneComponent.K2_GetComponentLocation` _staticmesh) (* (`KismetMathLibrary.GetForwardVector` _returnvalue) 50.0)) (select `bool` (`self.tircentre`) :`false` (`KismetMathLibrary.FindLookAtRotation` (`self.DeprojectMousePositionToWorld`) (select `bool` (>= (/ (`/Game/game/player/df_pawn_bp.speed` _asdf_pawn_bp) (`/Game/game/player/df_pawn_bp.speedmax` _asdf_pawn_bp)) 0.5) :`false` _returnvalue_2 :`true` (- _returnvalue_2 (* (`SceneComponent.GetForwardVector` _camera) 5.0)))) :`true` _returnvalue)))
          (`GameplayStatics.PlaySound2D` "/Game/assets/sounds/enemy_laser.enemy_laser"))))))

(event `Key|LeftMouseButton`
  (params (Key :type "Key Structure" :default "AnyKey"))
  ;[0.2484 0.1438 1] fire on left mouse click
  (:`Pressed`
    (goto _label_2 :!via `Open`))
  (:`Released`
    (goto _label_2 :!via `Close`)))

(event `fireserver_Event`
  (params (val :type "Transform Structure"))
  (bind _returnvalue (`self.K2_GetPawn`))
  ;[0.2484 0.1438 1] fire on left mouse click
  (bind _returnvalue_2 (`|SpawnActorFromClass` "/Game/game/green_bullet_bp.green_bullet_bp_C" val "AlwaysSpawn" "OverrideRootScale" _returnvalue))
  (set `/Game/game/green_bullet_bp.ownerShip` _returnvalue _returnvalue_2))

(event `destroy_pawn`
  ;[1 1 1] destroy pawn
  (bind _returnvalue (`|CreateWidget` "/Game/game/ui/ui_death_widget.ui_death_widget_C" self))
  (`UserWidget.AddToViewport` _returnvalue 0)
  (set `self.bShowMouseCursor` true))

(event `Key|Escape`
  (params (Key :type "Key Structure" :default "AnyKey"))
  ;[1 0 0] Quit Game
  (:`Pressed`
    (`KismetSystemLibrary.QuitGame` self "Quit")))

(fn `UserConstructionScript`)