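; Space station Blueprint meant to show a station UI widget on right mouse button release.
; Releasing the button adds the stored Stationwidget to the viewport.
; The logic that enables input, creates the Stationui widget and fills its name label from the station's Name is disconnected and never runs, so nothing here assigns that widget.
; BeginPlay and the construction script are empty.
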(event `self.ReceiveBeginPlay`)

(event `Key|RightMouseButton`
  (params (Key :type "Key Structure" :default "AnyKey"))
  (:`Released`
    (`UserWidget.AddToViewport` (`self.stationwidget`) 0)))

(fn `UserConstructionScript`)