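; Red bullet projectile that damages player pawns, AI pawns and gopoint actors it overlaps.
; On authority, overlaps with actors other than itself and its owner cast to each type, call its damage function and multicast an explosion effect and sound at the target.
; Other actors get only the explosion.
; Tick on authority destroys the bullet after a ten-second lifetime; the overlap path itself does not destroy it.
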(event `overlap_server`
  (`self.K2_DestroyActor` self))

(event `self.ReceiveActorBeginOverlap`
  (params (OtherActor :type "Actor Object Reference"))
  (`/Engine/EditorBlueprintResources/ActorMacros.Switch Has Authority`
    (:`Authority`
      ;[0.358 1 0.2646] Different from owner, and itself
      (if (!= OtherActor self)
        (if (!= (`self.GetOwner` self) OtherActor)
          (bind _asdf_pawn_bp (cast `/Game/game/player/df_pawn_bp` OtherActor)
            (:`then`
              (`self.overlap_mutlicast` (`SceneComponent.K2_GetComponentLocation` (`/Game/game/player/df_pawn_bp.StaticMesh` _asdf_pawn_bp)))
              (`/Game/game/player/df_pawn_bp.Take Damage` _asdf_pawn_bp self))
            (:`CastFailed`
              (bind _asdf_pawnai_bp (cast `/Game/game/AI/df_pawnai_bp` OtherActor)
                (:`then`
                  (`self.overlap_mutlicast` (`SceneComponent.K2_GetComponentLocation` (`/Game/game/AI/df_pawnai_bp.StaticMesh` _asdf_pawnai_bp)))
                  (`/Game/game/AI/df_pawnai_bp.Take Damage` _asdf_pawnai_bp self))
                (:`CastFailed`
                  (bind _asgopoint (cast `/Game/game/zone/gopoint` OtherActor)
                    (:`then`
                      (`self.overlap_mutlicast` (`SceneComponent.K2_GetComponentLocation` (`/Game/game/zone/gopoint.StaticMesh` _asgopoint)))
                      (`/Game/game/zone/gopoint.takedamage` _asgopoint self))
                    (:`CastFailed`
                      (`self.overlap_mutlicast` (`self.K2_GetActorLocation` OtherActor)))))))))))))

(event `overlap_mutlicast`
  (params (locaiton :type "Vector Structure"))
  ;[1 0.8063 0.1441] while overlap create explosion
  (`GameplayStatics.SpawnEmitterAtLocation` "/Game/StarterContent/Particles/P_Explosion.P_Explosion" locaiton)
  (`GameplayStatics.SpawnSoundAtLocation` "/Game/assets/sounds/Blast-SoundBible.Blast-SoundBible" locaiton))

(event `self.ReceiveBeginPlay`
  (set `self.lifeStart` (`GameplayStatics.GetRealTimeSeconds`)))

(event `self.ReceiveTick`
  (params (DeltaSeconds :type "Float (single-precision)"))
  (`/Engine/EditorBlueprintResources/ActorMacros.Switch Has Authority`
    (:`Authority`
      (if (> (- (`GameplayStatics.GetRealTimeSeconds`) (`self.lifeStart`)) 10.0)
        (`self.K2_DestroyActor` self)))))

(fn `UserConstructionScript`)