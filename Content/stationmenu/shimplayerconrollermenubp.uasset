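; Player controller for the station menu that creates the station widget on BeginPlay and switches between mission list and single mission views.
; Changestatus stores the requested state and mission Id, removing the tiny mission widgets when leaving the shown list.
; Tick polls the status string as a simple state machine, calls ShowListMissions or ShowMission on the first ShimStation actor, then marks that view as shown.
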(event `self.ReceiveBeginPlay`
  (bind _returnvalue (`|CreateWidget` "/Game/stationmenu/stationwidget.stationwidget_C" self))
  (`UserWidget.AddToViewport` _returnvalue 0))

(event `self.ReceiveTick`
  (params (DeltaSeconds :type "Float (single-precision)"))
  (bind _status (`self.status`))
  (if (`KismetStringLibrary.EqualEqual_StrStr` _status "showlistmission")
    (bind _outactors (`GameplayStatics.GetAllActorsOfClass` "/Script/pocshim.ShimStation"))
    (`ShimStation.ShowListMissions` (`KismetArrayLibrary.Array_Get` _outactors))
    (set `self.status` "listofmissionshown")
    (elif (`KismetStringLibrary.EqualEqual_StrStr` _status "showmission")
      (bind _outactors_2 (`GameplayStatics.GetAllActorsOfClass` "/Script/pocshim.ShimStation"))
      (`ShimStation.ShowMission` (`KismetArrayLibrary.Array_Get` _outactors_2) (`self.id`))
      (set `self.status` "missionshown"))))

(fn `changestatus`
  (params (newstatus :type String) (id :type Integer))
  (set `self.id` id)
  (if (`KismetStringLibrary.EqualEqual_StrStr` (`self.status`) "listofmissionshown")
    (bind _foundwidgets (`WidgetBlueprintLibrary.GetAllWidgetsOfClass` "/Game/stationmenu/tinymissionwidgetbp.tinymissionwidgetbp_C" false))
    (for _array_element _foundwidgets
      (`Widget.RemoveFromParent` _array_element)))
  (set `self.status` newstatus))

(fn `UserConstructionScript`)