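; Networked bullet projectile that explodes on hitting ships and pawns, with lifetime and collisions handled on the server.
; It records its spawn time and destroys itself on Tick after a fixed lifetime.
; Overlaps ignore the owner, call TakeDamage on a mainship_bp, and destroy the bullet only on a mainpawn_bp hit.
; Both hit types trigger a multicast event that spawns explosion particles and sound at the target's mesh location.
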(event `self.ReceiveBeginPlay`
  ;[0.2746 0.1989 1] beginplay : time of starting life of the bullet
  (set `self.lifeStart` (`GameplayStatics.GetRealTimeSeconds`)))

(event `overlap_server`
  (`self.K2_DestroyActor` self))

(event `self.ReceiveTick`
  (params (DeltaSeconds :type "Float (single-precision)"))
  ;[1 0.2581 0.2294] DEstroy bullet over time
  (`/Engine/EditorBlueprintResources/ActorMacros.Switch Has Authority`
    (:`Authority`
      (if (> (- (`GameplayStatics.GetRealTimeSeconds`) (`self.lifeStart`)) 10.0)
        (`self.K2_DestroyActor` self)))))

(event `overlap_mutlicast`
  (params (locaiton :type "Vector Structure"))
  ;[1 0.8063 0.1441] while overlap create explosion
  (`GameplayStatics.SpawnEmitterAtLocation` "/Game/StarterContent/Particles/P_Explosion.P_Explosion" locaiton)
  (`GameplayStatics.SpawnSoundAtLocation` "/Game/assets/sounds/Blast-SoundBible.Blast-SoundBible" locaiton))

(event `self.ReceiveActorBeginOverlap`
  (params (OtherActor :type "Actor Object Reference"))
  (`/Engine/EditorBlueprintResources/ActorMacros.Switch Has Authority`
    (:`Authority`
      ;[0.358 1 0.2646] Different from owner, and itself
      (if (!= OtherActor self)
        (if (!= (`self.GetOwner` self) OtherActor)
          ;[0.06128 1 0] shoot on ship
          (bind _asmainship_bp (cast `/Game/bp/mainship_bp` OtherActor)
            (:`then`
              (`/Game/bp/mainship_bp.Take Damage` _asmainship_bp self)
              (`self.overlap_mutlicast` (`SceneComponent.K2_GetComponentLocation` (`/Game/bp/mainpawn_bp.StaticMesh` _asmainship_bp))))
            (:`CastFailed`
              ;[0 1 0.5103] shoot on other pawn
              (bind _asmainpawn_bp (cast `/Game/bp/mainpawn_bp` OtherActor))
              (`self.overlap_mutlicast` (`SceneComponent.K2_GetComponentLocation` (`/Game/bp/mainpawn_bp.StaticMesh` _asmainpawn_bp)))
              (`self.K2_DestroyActor`))))))))

(fn `UserConstructionScript`)